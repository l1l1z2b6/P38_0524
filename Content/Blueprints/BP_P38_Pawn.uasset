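; P-38 plane pawn that the player flies with roll and pitch axis inputs.
; Tick spins the left and right propeller components at their own speeds and constantly adds full forward movement input along the actor's facing.
; The Roll and Pitch inputs apply local actor rotation at a fixed rate scaled by delta time, so steering is relative to the plane's orientation.
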(event `self.ReceiveTick`
  (params (DeltaSeconds :type "Float (single-precision)"))
  (`|ExecutionSequence`
    (:`then_0`
      (`self.Propeller L`))
    (:`then_1`
      (`self.Propeller R`))
    (:`then_2`
      (`self.AddMovementInput` (`self.GetActorForwardVector`)))))

(event `InputAxis|Roll`
  (params (AxisValue :type "Float (single-precision)"))
  (`self.Roll` AxisValue))

(event `InputAxis|Pitch`
  (params (AxisValue :type "Float (single-precision)"))
  (`self.Pitch` AxisValue))

(fn `Pitch`
  (params (A :type "Float (double-precision)"))
  (`self.K2_AddActorLocalRotation` (`KismetMathLibrary.MakeRotator` 0.0 (* A 60.0 (`GameplayStatics.GetWorldDeltaSeconds`)))))

(fn `Propeller L`
  (`SceneComponent.K2_AddLocalRotation` (`self.Propeller_L`) (`KismetMathLibrary.MakeRotator` (* (`GameplayStatics.GetWorldDeltaSeconds`) (`self.PropellerSpeed_L`))) false false))

(fn `Propeller R`
  (`SceneComponent.K2_AddLocalRotation` (`self.Propeller_R`) (`KismetMathLibrary.MakeRotator` (* (`GameplayStatics.GetWorldDeltaSeconds`) (`self.PropellerSpeed_R`))) false false))

(fn `Roll`
  (params (A :type "Float (double-precision)"))
  (`self.K2_AddActorLocalRotation` (`KismetMathLibrary.MakeRotator` (* A 60.0 (`GameplayStatics.GetWorldDeltaSeconds`)))))

(fn `UserConstructionScript`)